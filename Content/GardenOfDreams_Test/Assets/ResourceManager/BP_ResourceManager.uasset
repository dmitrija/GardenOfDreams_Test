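; BP_ResourceManager is a Blueprint that holds a resource count and can transfer amounts to another manager.
; SetCount clamps the value between zero and MaxCount, fires OnUpdateCount with new and previous values only on change, and returns the amount that did not fit.
; AddCount applies a relative change through SetCount.
; Transite offers no more than CurrentCount to the target and deducts only what it accepted.
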(event EventBeginPlay)

(event Collision|EventActorBeginOverlap
  (params (OtherActor :type Actor%20Object%20Reference)))

(event EventTick
  (params (DeltaSeconds :type Float%20%28single-precision%29)))

(fn ConstructionScript)

(fn SetCount
  (params (NewCount :type Integer))
  (Utilities|FlowControl|Sequence
    (:then_0
      (LocalVariables|SetLocal_TargetCount (Math|Integer|Clamp(Integer) NewCount 0 (Variables|Default|GetMaxCount)))
      (if (!= (LocalVariables|GetLocal_TargetCount) (Variables|Default|GetCurrentCount))
        (LocalVariables|SetLocal_PrevCount (Variables|Default|GetCurrentCount))
        (bind _output_get (Variables|Default|SetCurrentCount (LocalVariables|GetLocal_TargetCount)))
        (Default|CallOnUpdateCount _output_get (LocalVariables|GetLocal_PrevCount))))
    (:then_1
      (return (- NewCount (Variables|Default|GetCurrentCount))))))

(fn AddCount
  (params (Count :type Integer))
  (bind _remainder (CallFunction|SetCount (+ Count (Variables|Default|GetCurrentCount))))
  (return _remainder))

(fn Transite
  (params (Count :type Integer) (TargetManager :type BP%20Resource%20Manager%20Object%20Reference))
  (bind _output_get (LocalVariables|SetLocal_ClampedCount (Math|Integer|Clamp(Integer) Count 0 (Variables|Default|GetCurrentCount))))
  (bind _remainder (CallFunction|AddCount TargetManager _output_get))
  (CallFunction|AddCount (* (- (LocalVariables|GetLocal_ClampedCount) _remainder) -1)))